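; Enemy spawner that toggles a group of enemies on and off as the player crosses its Trigger and Destroyer volumes.
; Spawning creates set numbers of chase and random AI enemies at random points inside the Spawner box and reveals the PathEnemies, which start hidden.
; Despawning destroys and clears the tracked spawned enemies and runs a hide pass.
; Both volumes flip the shared Spawned flag, so either can spawn or despawn.
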(event OnComponentBeginOverlap(Trigger)
  (params (OverlappedComponent :type Primitive%20Component%20Object%20Reference) (OtherActor :type Actor%20Object%20Reference) (OtherComp :type Primitive%20Component%20Object%20Reference) (OtherBodyIndex :type Integer) (bFromSweep :type Boolean) (SweepResult :type Hit%20Result%20Structure%20%28by%20ref%29))
  ;[1 1 1] TriggerBeginOverlap
  (if (Actor|ActorHasTag OtherActor "Player")
    (if (not (Variables|Default|GetSpawned))
      (CallFunction|BeginSpawn)
      (Variables|Default|SetSpawned true)
      (else
        (CallFunction|DestroyEnemies)
        (Variables|Default|SetSpawned false)))))

(event OnComponentBeginOverlap(Destroyer)
  (params (OverlappedComponent :type Primitive%20Component%20Object%20Reference) (OtherActor :type Actor%20Object%20Reference) (OtherComp :type Primitive%20Component%20Object%20Reference) (OtherBodyIndex :type Integer) (bFromSweep :type Boolean) (SweepResult :type Hit%20Result%20Structure%20%28by%20ref%29))
  ;[1 1 1] DestroyerBeginOverlap
  (if (Actor|ActorHasTag OtherActor "Player")
    (if (Variables|Default|GetSpawned)
      (CallFunction|DestroyEnemies)
      (Variables|Default|SetSpawned false)
      (else
        (CallFunction|BeginSpawn)
        (Variables|Default|SetSpawned true)))))

(event Custom|SpawnEnemies
  (params (EnemyType :type Pawn%20Class%20Reference))
  (bind _spawner (Variables|Default|GetSpawner))
  ;[1 1 1] Spawn
  (bind _returnvalue (AI|SpawnAIFromClass EnemyType 0 (Math|Random|RandomPointinBoundingBox (Transformation|GetWorldLocation _spawner) (Components|Box|GetScaledBoxExtent _spawner)) "0, 0, 0" false))
  (if (Utilities|IsValid _returnvalue)
    (Utilities|Array|Add (Variables|Default|GetEnemiesSpawned) _returnvalue)))

(event Custom|BeginSpawn
  ;[1 1 1] BeginSpawn
  (Utilities|FlowControl|Sequence
    (:then_0
      (for _index (range 0 (- (Variables|Default|GetEnemyChaseToSpawn) 1))
        (CallFunction|SpawnEnemies "/Game/Blueprints/Enemies/BP_EnemyChase.BP_EnemyChase_C")))
    (:then_1
      (for _index_2 (range 0 (- (Variables|Default|GetEnemyRandomToSpawn) 1))
        (CallFunction|SpawnEnemies "/Game/Blueprints/Enemies/BP_EnemyRandom.BP_EnemyRandom_C")))
    (:then_2
      (for _array_element (Variables|Default|GetPathEnemies)
        (Rendering|SetActorHiddenInGame _array_element false)))))

(event Custom|DestroyEnemies
  (bind _enemiesspawned (Variables|Default|GetEnemiesSpawned))
  ;[1 1 1] DestroySpawned
  (Utilities|FlowControl|Sequence
    (:then_0
      (for _array_element _enemiesspawned
        (Actor|DestroyActor _array_element))
      (Utilities|Array|Clear _enemiesspawned))
    (:then_1
      (for _array_element_2 0
        (Rendering|SetActorHiddenInGame _array_element_2 true)))))

(event EventBeginPlay
  ;[1 1 1] Hide add enemies at the beginning
  (for _array_element (Variables|Default|GetPathEnemies)
    (Rendering|SetActorHiddenInGame _array_element true)))

(fn ConstructionScript)