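; Enemy AI controller that picks a movement behaviour on possession from the controlled character's EnemyType: chase, patrol, patrol-chase or random wander.
; Chasers re-issue AIMoveTo toward the player, while patrollers step through spline points and wrap around, advancing even when a move fails.
; Patrol-chasers switch to pursuing the player within a spotting distance, checked whenever a move ends or after a delay while chasing.
; Wanderers move to random reachable points on a looping timer.
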(event Custom|TrackPlayer
  ;[1 1 1] Track Player AI
  (AI|AIMoveTo (Pawn|GetControlledPawn) "0, 0, 0" (Game|GetPlayerCharacter 0) 5.0 false
    (:OnSuccess
      _)
    (:OnFail
      _))
  (CallFunction|TrackPlayer))

(event Custom|PatrolChase
  (bind _returnvalue (Game|GetPlayerCharacter 0))
  (bind _returnvalue_2 (Pawn|GetControlledPawn))
  (bind _enemypatrolchase (Variables|Default|GetEnemyPatrolChase))
  ;[1 1 1] PatrolChase
  (if (<= (Transformation|GetDistanceTo _returnvalue_2 _returnvalue) (Variables|Default|GetMinimalSpottedDistance))
    (AI|AIMoveTo _returnvalue_2 "0, 0, 0" _returnvalue 5.0 false
      (:then
        (Utilities|FlowControl|Delay 2.0)
        (CallFunction|PatrolChase)))
    (else
      (AI|AIMoveTo _enemypatrolchase (Spline|GetLocationatSplinePoint (Variables|/Game/Blueprints/Enemies/BP_EnemyCharacter.BP_EnemyCharacter_C|GetPath _enemypatrolchase) (Variables|/Game/Blueprints/Enemies/BP_EnemyCharacter.BP_EnemyCharacter_C|GetSplineIndex _enemypatrolchase) "World") 0 5.0 false
        (:OnSuccess
          _)
        (:OnFail
          _))
      (if (== (Variables|/Game/Blueprints/Enemies/BP_EnemyCharacter.BP_EnemyCharacter_C|GetSplineIndex _enemypatrolchase) (Variables|/Game/Blueprints/Enemies/BP_EnemyCharacter.BP_EnemyCharacter_C|GetMaxSplinePoints _enemypatrolchase))
        (Variables|/Game/Blueprints/Enemies/BP_EnemyCharacter.BP_EnemyCharacter_C|SetSplineIndex _enemypatrolchase 0)
        (else
          (Math|Integer|IncrementInt (Variables|/Game/Blueprints/Enemies/BP_EnemyCharacter.BP_EnemyCharacter_C|GetSplineIndex _enemypatrolchase)
            (:%20%20
              _))))
      (CallFunction|PatrolChase))))

(event Custom|PatrolWalk
  (bind _enemypatrol (Variables|Default|GetEnemyPatrol))
  ;[1 1 1] PatrolWalk
  (AI|AIMoveTo _enemypatrol (Spline|GetLocationatSplinePoint (Variables|/Game/Blueprints/Enemies/BP_EnemyCharacter.BP_EnemyCharacter_C|GetPath _enemypatrol) (Variables|/Game/Blueprints/Enemies/BP_EnemyCharacter.BP_EnemyCharacter_C|GetSplineIndex _enemypatrol) "World") 0 5.0 false
    (:OnSuccess
      _)
    (:OnFail
      _))
  (if (== (Variables|/Game/Blueprints/Enemies/BP_EnemyCharacter.BP_EnemyCharacter_C|GetSplineIndex _enemypatrol) (Variables|/Game/Blueprints/Enemies/BP_EnemyCharacter.BP_EnemyCharacter_C|GetMaxSplinePoints _enemypatrol))
    (Variables|/Game/Blueprints/Enemies/BP_EnemyCharacter.BP_EnemyCharacter_C|SetSplineIndex _enemypatrol 0)
    (else
      (Math|Integer|IncrementInt (Variables|/Game/Blueprints/Enemies/BP_EnemyCharacter.BP_EnemyCharacter_C|GetSplineIndex _enemypatrol)
        (:%20%20
          _))))
  (CallFunction|PatrolWalk))

(event Custom|WalkRandom
  (bind _returnvalue (Pawn|GetControlledPawn))
  ;[1 1 1] WalkRandom
  (AI|AIMoveTo _returnvalue (.RandomLocation (AI|Navigation|GetRandomReachablePointinRadius (Transformation|GetActorLocation _returnvalue) 2e+04 0 0)) 0 5.0 false))

(event EventPossess
  (params (PossessedPawn :type Pawn%20Object%20Reference))
  (bind _returnvalue (Pawn|GetControlledPawn))
  ;[1 1 1] Setup references to possible AI
  (switch Utilities|FlowControl|Switch|SwitchonE_EnemyType (Variables|/Game/Blueprints/Enemies/BP_EnemyCharacter.BP_EnemyCharacter_C|GetEnemyType (.AsBP%20Enemy%20Character (Utilities|Casting|CastToBP_EnemyCharacter _returnvalue)))
    (:NewEnumerator0
      (bind _asbp_enemy_chase (Utilities|Casting|CastToBP_EnemyChase _returnvalue))
      (Variables|Default|SetEnemyChase _asbp_enemy_chase)
      (CallFunction|TrackPlayer))
    (:NewEnumerator1
      (bind _asbp_enemy_patrol (Utilities|Casting|CastToBP_EnemyPatrol _returnvalue))
      (Variables|Default|SetEnemyPatrol _asbp_enemy_patrol)
      (CallFunction|PatrolWalk))
    (:NewEnumerator2
      (bind _asbp_enemy_patrol_chase (Utilities|Casting|CastToBP_EnemyPatrolChase _returnvalue))
      (Variables|Default|SetEnemyPatrolChase _asbp_enemy_patrol_chase)
      (CallFunction|PatrolChase))
    (:NewEnumerator3
      (bind _asbp_enemy_random (Utilities|Casting|CastToBP_EnemyRandom _returnvalue))
      (Variables|Default|SetEnemyRandom _asbp_enemy_random)
      (Utilities|Time|SetTimerbyFunctionName 0 "WalkRandom" 5.0 true))))

(fn ConstructionScript)